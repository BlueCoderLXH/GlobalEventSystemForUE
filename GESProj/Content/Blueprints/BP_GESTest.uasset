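; BP_GESTest is a test Blueprint that checks receipt of a map payload through a global event system (GES).
; On BeginPlay it registers a listener for "MapTestEvent" and routes the received map to OnMapTest.
; OnMapTest prints each key-value pair between start and end messages, through a PrintMsg helper that adds the asset name.
; GetModuleName returns "Test.BP_GESTest", which suggests a script module binding such as UnLua.
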(event `self.ReceiveBeginPlay`
  (bind _eventdata0 (`|GESRegisterEvent` "MapTestEvent")
    (:`OnEvent`
      (`self.OnMapTest` _eventdata0))))

(fn `GetModuleName`
  (returns (ReturnValue :type String))
  (return "Test.BP_GESTest"))

(fn `OnMapTest`
  (params (InMapData :type "Map of Integer to Vector Structure"))
  (`|ExecutionSequence`
    (:`then_0`
      (`self.PrintMsg` "Receive 'MapTestEvent' Start"))
    (:`then_1`
      (bind _keys (`BlueprintMapLibrary.Map_Keys` (`local.InMapData`)))
      (for _array_element _keys
        (`self.PrintMsg` (`KismetStringLibrary.Concat_StrStr` "Map[" (`KismetStringLibrary.Conv_IntToString` _array_element) "]=" (`KismetStringLibrary.Conv_VectorToString` (`BlueprintMapLibrary.Map_Find` (`local.InMapData`) _array_element))))))
    (:`then_2`
      (`self.PrintMsg` "Receive 'MapTestEvent' End"))))

(fn `PrintMsg`
  (params (Msg :type String))
  (`KismetSystemLibrary.PrintString` (`KismetStringLibrary.Concat_StrStr` "[BP_GESTest] " Msg)))

(fn `UserConstructionScript`)